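; Openable door Blueprint that swings the actor open and closed in response to OnOpen and OnClose events from its OpenDoor component.
; It caches the initial rotation on BeginPlay, then plays or reverses the DoorSwing timeline to add an animated yaw offset to that rotation.
; An event track on the timeline plays the Doorlock sound at the door's location.
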(event OnOpen(OpenDoor)
  (bind _open_angle (Timeline|DoorSwing Play)
    (:Update
      (Transformation|SetActorRotation (Math|Rotator|CombineRotators (Variables|Default|GetInitial%20Rotation) (Math|Rotator|MakeRotator 0.0 0.0 _open_angle))))
    (:Sound%20Timing
      (Audio|PlaySoundatLocation "/Game/Audio/door-lock.door-lock" (Transformation|GetActorLocation)))))

(event OnClose(OpenDoor)
  (bind _open_angle (Timeline|DoorSwing Reverse)
    (:Update
      (Transformation|SetActorRotation (Math|Rotator|CombineRotators (Variables|Default|GetInitial%20Rotation) (Math|Rotator|MakeRotator 0.0 0.0 _open_angle))))
    (:Sound%20Timing
      (Audio|PlaySoundatLocation "/Game/Audio/door-lock.door-lock" (Transformation|GetActorLocation)))))

(event EventBeginPlay
  (Variables|Default|SetInitial%20Rotation (Transformation|GetActorRotation)))

(fn ConstructionScript)